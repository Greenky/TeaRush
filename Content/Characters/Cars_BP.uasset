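; Cars_BP is a looping traffic actor that drives a toon car along its local X axis between Start and End components.
; BeginPlay picks a random speed, and Tick offsets the car by that amount every frame, without delta-time scaling.
; On passing End's X, the car snaps back to Start's X, rerolls its speed and swaps one material slot to a random entry from Materials.
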(event `self.ReceiveBeginPlay`
  (set `self.RandomSpeed` (`KismetMathLibrary.RandomFloatInRange` 20.0 50.0)))

(event `self.ReceiveTick`
  (params (DeltaSeconds :type "Float (single-precision)"))
  (bind _toon_car_1 (`self.toon_car_1`))
  (bind (_relativelocation_x _relativelocation_y _relativelocation_z) (`KismetMathLibrary.BreakVector` (`SceneComponent.RelativeLocation` _toon_car_1)))
  (bind _relativelocation_x_2 (`KismetMathLibrary.BreakVector` (`SceneComponent.RelativeLocation` (`self.Start`))))
  (bind _relativelocation_x_3 (`KismetMathLibrary.BreakVector` (`SceneComponent.RelativeLocation` (`self.toon_car_1`))))
  (bind _relativelocation_x_4 (`KismetMathLibrary.BreakVector` (`SceneComponent.RelativeLocation` (`self.End`))))
  (`SceneComponent.K2_AddLocalOffset` (`self.toon_car_1`) (`KismetMathLibrary.MakeVector` (`self.RandomSpeed`)) false false)
  (if (>= _relativelocation_x_3 _relativelocation_x_4)
    (`SceneComponent.K2_SetRelativeLocation` _toon_car_1 (`KismetMathLibrary.MakeVector` _relativelocation_x_2 _relativelocation_y _relativelocation_z) false false)
    (set `self.RandomSpeed` (`KismetMathLibrary.RandomFloatInRange` 20.0 50.0))
    (`PrimitiveComponent.SetMaterial` (`self.toon_car_1`) 1 (`|GetArrayItem` (`self.Materials`) (`KismetMathLibrary.RandomIntegerInRange` 0 3)))))

(fn `UserConstructionScript`)