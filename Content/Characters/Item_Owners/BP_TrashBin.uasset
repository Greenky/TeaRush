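; BP_TrashBin is an item-owner Blueprint for a trash bin that extends the parent's item menu with a "Clean" button.
; OpenMenu creates a WB_CalbackButton, adds it to the menu's bottom panel and binds an event to it.
; OnAdded, OnRemoved and ClearItems overrides keep the button enabled only while the bin holds items.
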(fn `Add Bottom Panel To Menu`
  (params (Widget :type "Widget Object Reference"))
  (`/Engine/EditorBlueprintResources/StandardMacros.IsValid` (`self.Item Menu`)
    (:`Is Valid`
      (`PanelWidget.AddChild` (`/Game/UI/WB_Inventory_Menu_Item_Owner.Button` (`self.Item Menu`)) Widget))))

(fn `Clear Items`
  (`parent.Clear Items`)
  (set `Widget.bIsEnabled` false (`self.Button`)))

(fn `On Added`
  (params (Item :type "/Game/TopDown/Items/BP_Food_Item Object Reference"))
  (`parent.On Added` Item)
  (set `Widget.bIsEnabled` true (`self.Button`)))

(fn `On Removed`
  (params (Item :type "/Game/TopDown/Items/BP_Food_Item Object Reference"))
  (`parent.On Removed` Item)
  (set `Widget.bIsEnabled` (`KismetArrayLibrary.Array_IsNotEmpty` (`self.Owned Items`)) (`self.Button`)))

(fn `Open Menu`
  (`parent.Open Menu`)
  (bind _returnvalue (`|CreateWidget` "/Game/UI/InventoryElements/WB_CalbackButton.WB_CalbackButton_C" null "Clean"))
  (`self.Add Bottom Panel To Menu` _returnvalue)
  (add `/Game/UI/InventoryElements/WB_CalbackButton.Action` _returnvalue (`|CreateDelegate` :!event `Clear Items`))
  (bind _output_get (set `self.Button` _returnvalue))
  (set `Widget.bIsEnabled` (`KismetArrayLibrary.Array_IsNotEmpty` (`self.Owned Items`)) _output_get))

(fn `UserConstructionScript`
  (`parent.UserConstructionScript`))