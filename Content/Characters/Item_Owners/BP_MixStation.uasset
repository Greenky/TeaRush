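; Mixing station item owner that combines the items it holds into a food item using the game mode's available recipes.
; OpenMenu extends the parent menu with a "Mix" callback button in the bottom panel.
; Mix gathers item types into a gameplay tag container and takes the first recipe whose ingredients are all present.
; That match replaces all held items with the resulting BP_Food_Item and refreshes the menu list.
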(fn `Add Bottom Panel To Menu`
  (params (Widget :type "Widget Object Reference"))
  (`/Engine/EditorBlueprintResources/StandardMacros.IsValid` (`self.Item Menu`)
    (:`Is Valid`
      (`PanelWidget.AddChild` (`/Game/UI/WB_Inventory_Menu_Item_Owner.Button` (`self.Item Menu`)) Widget))))

(fn `Mix`
  (locals (Ingredients :type "GameplayTagContainer Structure"))
  (bind _asbp_top_down_game_mode (cast `/Game/TopDown/Blueprints/BP_TopDownGameMode` (`GameplayStatics.GetGameMode`)))
  (for _array_element (`self.Owned Items`)
    (`BlueprintGameplayTagLibrary.AddGameplayTag` (`local.Ingredients`) (`/Game/TopDown/Items/BP_Food_Item.Type` _array_element)))
  (for _array_element_2 (`/Game/TopDown/Blueprints/BP_TopDownGameMode.Get Available Recipes` _asbp_top_down_game_mode)
    (bind (_result _ingredients) (break `/Game/TopDown/Items/S_Recipe` _array_element_2))
    (if (`BlueprintGameplayTagLibrary.HasAllTags` (`local.Ingredients`) _ingredients true)
      (bind _returnvalue (`|GenericCreateObject` "/Game/TopDown/Items/BP_Food_Item.BP_Food_Item_C" _result))
      (`self.Clear Items`)
      (`KismetArrayLibrary.Array_Add` (`self.Owned Items`) _returnvalue)
      (`self.Reset Menu List`)
      (break))))

(fn `Open Menu`
  (`parent.Open Menu`)
  (bind _returnvalue (`|CreateWidget` "/Game/UI/InventoryElements/WB_CalbackButton.WB_CalbackButton_C" null "Mix"))
  (`self.Add Bottom Panel To Menu` _returnvalue)
  (add `/Game/UI/InventoryElements/WB_CalbackButton.Action` _returnvalue (`|CreateDelegate` :!event `Mix`)))

(fn `UserConstructionScript`
  (`parent.UserConstructionScript`))