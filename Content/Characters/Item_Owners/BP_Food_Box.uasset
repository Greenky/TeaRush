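; BP_Food_Box is an item owner that acts as a source of food items.
; It reports that it can create any type under the Item.Food gameplay tag, including child tags.
; Creating an item looks up the type in the game mode's CookableStages map and, if found, constructs a BP_Food_Three_State with those stages and that type.
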(fn `Can Create Item`
  (params (Type :type "GameplayTag Structure"))
  (returns (Result :type Boolean))
  (return (`BlueprintGameplayTagLibrary.MatchesTag` Type (struct :`TagName` "Item.Food"))))

(fn `Create Item`
  (params (Type :type "GameplayTag Structure"))
  (returns (item :type "/Game/TopDown/Items/BP_Food_Item Object Reference"))
  (bind _asbp_top_down_game_mode (cast `/Game/TopDown/Blueprints/BP_TopDownGameMode` (`GameplayStatics.GetGameMode`)))
  (bind (_value _returnvalue) (`BlueprintMapLibrary.Map_Find` (`/Game/TopDown/Blueprints/BP_TopDownGameMode.Cookable Stages` _asbp_top_down_game_mode) (`local.Type`)))
  (if _returnvalue
    (bind _returnvalue_2 (`|GenericCreateObject` "/Game/TopDown/Items/BP_Food_Three_State.BP_Food_Three_State_C" _value (`local.Type`)))
    (return _returnvalue_2)))

(fn `UserConstructionScript`
  (`parent.UserConstructionScript`))