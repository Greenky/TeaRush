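; Item box, an item owner that holds a stock of items and shows them in its own inventory menu widget.
; BeginPlay tries to create each InitialItems entry, and Tick tops up with random picks from that list while fewer than twelve are owned.
; TryCreateItem adds created items to OwnedItems and the menu.
; CanCreateItem always allows creation, while CreateItem has an empty body here.
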(event `self.ReceiveBeginPlay`
  (for _array_element (`self.Initial items`)
    (`self.Try Create Item` _array_element)
    (`parent.ReceiveBeginPlay`)))

(event `self.ReceiveTick`
  (params (DeltaSeconds :type "Float (single-precision)"))
  (`parent.ReceiveTick` DeltaSeconds)
  (if (and (`KismetArrayLibrary.Array_IsNotEmpty` (`self.Initial items`)) (< (`KismetArrayLibrary.Array_Length` (`self.Owned Items`)) 12))
    (`self.Try Create Item` (`KismetArrayLibrary.Array_Random` (`self.Initial items`)))))

(fn `Can Create Item`
  (params (Type :type "GameplayTag Structure"))
  (returns (Result :type Boolean))
  (return true))

(fn `Create Item`
  (params (Type :type "GameplayTag Structure"))
  (returns (item :type "/Game/TopDown/Items/BP_Food_Item Object Reference")))

(fn `Create Menu`
  (returns (ReturnValue :type "/Game/UI/WB_Inventory_Menu_Item_Owner Object Reference"))
  (bind _returnvalue (`|CreateWidget` "/Game/UI/WB_Inventory_Menu_ItemBox.WB_Inventory_Menu_ItemBox_C" null self))
  (return _returnvalue))

(fn `Try Create Item`
  (params (Type :type "GameplayTag Structure"))
  (if (`self.Can Create Item` Type)
    (bind _item (`self.Create Item` Type))
    (`KismetArrayLibrary.Array_Add` (`self.Owned Items`) _item)
    (`self.Add to Menu` _item)))

(fn `UserConstructionScript`
  (`parent.UserConstructionScript`))