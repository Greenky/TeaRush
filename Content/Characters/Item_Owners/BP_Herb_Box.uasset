(fn `Can Create Item`
  (params (Type :type "GameplayTag Structure"))
  (returns (Result :type Boolean))
  (return (`BlueprintGameplayTagLibrary.MatchesTag` Type (struct :`TagName` "Item.Herb"))))

(fn `Create Item`
  (params (Type :type "GameplayTag Structure"))
  (returns (item :type "/Game/TopDown/Items/BP_Food_Item Object Reference"))
  (bind _returnvalue (`|GenericCreateObject` "/Game/TopDown/Items/BP_Food_Item.BP_Food_Item_C" Type))
  (return _returnvalue))

(fn `UserConstructionScript`
  (`parent.UserConstructionScript`))