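; Clickable recipe book actor that shows a recipe menu widget in the player's HUD.
; It builds the list from the game mode's possible recipes, keeping those whose result is in the book's own Recipes list.
; Clicking within close range of the controlled pawn, or calling OpenMenu, replaces the HUD menu's content with that widget.
; CloseMenu removes only the widget stored by OpenMenu, as the click path does not save its widget.
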(event `self.ReceiveActorOnClicked`
  (params (ButtonPressed :type "Key Structure"))
  (bind _returnvalue (`GameplayStatics.GetPlayerController` 0))
  (if (<= (`self.GetDistanceTo` (`Controller.K2_GetPawn` _returnvalue) self) 300.0)
    (bind _asbp_hud (cast `/Game/UI/BP_HUD` (`PlayerController.GetHUD` _returnvalue)))
    (bind _returnvalue_2 (`|CreateWidget` "/Game/UI/WB_Recipe_Book.WB_Recipe_Book_C" null (`self.Get Recipes`)))
    (bind _menu (`/Game/UI/WB_HUD.Menu` (`/Game/UI/BP_HUD.HUD` _asbp_hud)))
    (`PanelWidget.ClearChildren` _menu)
    (`PanelWidget.AddChild` _menu _returnvalue_2)))

(fn `Close Menu`
  (`parent.Close Menu`)
  (if (`KismetSystemLibrary.IsValid` (`self.Item Menu`))
    (`Widget.RemoveFromParent` (`self.Item Menu`))))

(fn `Get Recipes`
  (returns (Result :type "Array of /Game/TopDown/Items/S_Recipe Structure"))
  (locals (`Recipes List` :type "Array of /Game/TopDown/Items/S_Recipe Structure"))
  (bind _asbp_top_down_game_mode (cast `/Game/TopDown/Blueprints/BP_TopDownGameMode` (`GameplayStatics.GetGameMode`)))
  (for _array_element (`/Game/TopDown/Blueprints/BP_TopDownGameMode.Possible Recipes` _asbp_top_down_game_mode)
    (if (`KismetArrayLibrary.Array_Contains` (`self.Recipes`) (`.Result_2_28C2311B443FB4E495C6578C18E4F696` (break `/Game/TopDown/Items/S_Recipe` _array_element)))
      (`KismetArrayLibrary.Array_Add` (`local.Recipes List`) _array_element)))
  (return (`local.Recipes List`)))

(fn `Open Menu`
  (`parent.Open Menu`)
  (bind _asbp_hud (cast `/Game/UI/BP_HUD` (`PlayerController.GetHUD` (`GameplayStatics.GetPlayerController` 0))))
  (bind _returnvalue (`|CreateWidget` "/Game/UI/WB_Recipe_Book.WB_Recipe_Book_C" null (`self.Get Recipes`)))
  (bind _output_get (set `self.Item Menu` _returnvalue))
  (bind _menu (`/Game/UI/WB_HUD.Menu` (`/Game/UI/BP_HUD.HUD` _asbp_hud)))
  (`PanelWidget.ClearChildren` _menu)
  (`PanelWidget.AddChild` _menu _output_get))

(fn `UserConstructionScript`
  (`parent.UserConstructionScript`))