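; BP_Table is an item-owner table where customers sit, order and get served for score.
; Customer overlap or a click fills an empty order with random available recipes, sized by difficulty.
; Its menu shows the order and a confirm button; confirming compares owned item tags to it.
; A match clears items, scores by tea/food tags times order length, re-registers the table with the spawner and sends the customer out; mismatches play a refusal sound.
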(event `self.ReceiveBeginPlay`
  (`parent.ReceiveBeginPlay`)
  (bind _asbp_game (cast `/Game/TopDown/Blueprints/BP_Game` (`GameplayStatics.GetGameInstance`)))
  (set `self.Game` _asbp_game))

(event `/Game/TopDown/Blueprints/BP_Interactable.ReceiveActorOnClicked`
  (params (ButtonPressed :type "Key Structure"))
  (`parent.ReceiveActorOnClicked` ButtonPressed)
  (`self.Create Order`))

(event `self.Box.OnComponentBeginOverlap`
  (params (OverlappedComponent :type "PrimitiveComponent Object Reference") (OtherActor :type "Actor Object Reference") (OtherComp :type "PrimitiveComponent Object Reference") (OtherBodyIndex :type Integer) (bFromSweep :type Boolean) (SweepResult :type "HitResult Structure (by ref)"))
  (bind (_returnvalue_x _returnvalue_y) (`KismetMathLibrary.BreakVector` (`SceneComponent.K2_GetComponentLocation` (`self.SittingSpot`))))
  (bind _asbp_customer (cast `/Game/TopDown/Blueprints/BP_Customer` OtherActor))
  (bind _output_get (set `self.Customer` _asbp_customer))
  (bind (_returnvalue_x_2 _returnvalue_y_2 _returnvalue_z) (`KismetMathLibrary.BreakVector` (`self.K2_GetActorLocation` _asbp_customer)))
  (`self.K2_SetActorLocationAndRotation` :`self` _output_get :`NewLocation` (`KismetMathLibrary.MakeVector` _returnvalue_x _returnvalue_y _returnvalue_z))
  (`self.Create Order`)
  (`GameplayStatics.PlaySoundAtLocation` "/Game/Music/hey-36263.hey-36263" (`self.K2_GetActorLocation` self) (struct) 1.0 1.0 0.0 null null null null))

(fn `Add Bottom Panel To Menu`
  (params (Widget :type "Widget Object Reference"))
  (`/Engine/EditorBlueprintResources/StandardMacros.IsValid` (`self.Item Menu`)
    (:`Is Valid`
      (`PanelWidget.AddChild` (`/Game/UI/WB_Inventory_Menu_Item_Owner.Button` (`self.Item Menu`)) Widget))))

(fn `Close Menu`
  (bind _orderview (`self.OrderView`))
  (`parent.Close Menu`)
  (if (`KismetSystemLibrary.IsValid` _orderview)
    (`Widget.RemoveFromParent` _orderview)))

(fn `Confirm Order`
  (locals (`Order To Confirm` :type "Array of GameplayTag Structure") (Failed :type Boolean) (LocalScore :type Integer))
  (bind _order (`self.Order`))
  (bind _gamemode (`self.GameMode`))
  (bind _localscore (`local.LocalScore`))
  (bind _returnvalue (`self.K2_GetActorLocation` self))
  (bind _asbp_top_down_game_mode (cast `/Game/TopDown/Blueprints/BP_TopDownGameMode` (`GameplayStatics.GetGameMode`)))
  (set `self.GameMode` _asbp_top_down_game_mode)
  (for _array_element (`self.Owned Items`)
    (`KismetArrayLibrary.Array_Add` (`local.Order To Confirm`) (`/Game/TopDown/Items/BP_Food_Item.Type` _array_element)))
  (for _array_element_2 (`self.Order`)
    (bind _returnvalue_2 (`KismetArrayLibrary.Array_Find` (`local.Order To Confirm`) _array_element_2))
    (if (!= _returnvalue_2 -1)
      (`KismetArrayLibrary.Array_Remove` (`local.Order To Confirm`) _returnvalue_2)
      (else
        (set `local.Failed` true)
        (break))))
  (if (and (`KismetArrayLibrary.Array_IsEmpty` (`local.Order To Confirm`)) (not (`local.Failed`)))
    (`self.Clear Items`)
    (if (`KismetSystemLibrary.IsValid` (`self.GameMode`))
      (set `local.LocalScore` 0)
      (for _array_element_3 _order
        (if (`BlueprintGameplayTagLibrary.MatchesTag` _array_element_3 (struct :`TagName` "Item.Tea"))
          (set `local.LocalScore` (+ 100 _localscore))
          (elif (`BlueprintGameplayTagLibrary.MatchesTag` _array_element_3 (struct :`TagName` "Item.Food"))
            (set `local.LocalScore` (+ 200 _localscore)))))
      (bind _output_get (set `local.LocalScore` (* (`local.LocalScore`) (`KismetArrayLibrary.Array_Length` _order))))
      (set `/Game/TopDown/Blueprints/BP_TopDownGameMode.Score` (+ _output_get (`/Game/TopDown/Blueprints/BP_TopDownGameMode.Score` _gamemode)) _gamemode)
      (set `local.LocalScore` 0)
      (`GameplayStatics.PlaySoundAtLocation` "/Game/Music/ScoreUP.ScoreUP" _returnvalue (struct) 1.0 1.0 0.0 null null null null)
      (`KismetArrayLibrary.Array_Clear` (`self.Order`)))
    (bind _outactors (`GameplayStatics.GetAllActorsOfClass` "/Game/TopDown/Blueprints/BP_CustomersSpawner.BP_CustomersSpawner_C"))
    (bind _output (`|GetArrayItem` _outactors))
    (`KismetArrayLibrary.Array_Add` (`/Game/TopDown/Blueprints/BP_CustomersSpawner.Tables` _output) self)
    (`/Game/TopDown/Blueprints/BP_Customer.EventMove` (`self.Customer`) (`SceneComponent.K2_GetComponentLocation` (`/Game/TopDown/Blueprints/BP_CustomersSpawner.Exit` _output)))
    (else
      (`GameplayStatics.PlaySoundAtLocation` (select `int` (`KismetMathLibrary.RandomIntegerInRange` 0 1) :`0` "/Game/Music/no-84725.no-84725" :`1` "/Game/Music/confused-what-103562.confused-what-103562" :!type "SoundBase Object Reference") _returnvalue (struct) 1.0 1.0 0.0 null null null null))))

(fn `Create Order`
  (if (`KismetArrayLibrary.Array_IsEmpty` (`self.Order`))
    (bind _asbp_top_down_game_mode (cast `/Game/TopDown/Blueprints/BP_TopDownGameMode` (`GameplayStatics.GetGameMode`)))
    (for _ (range (+ (`KismetMathLibrary.RandomIntegerInRange` 0 (select `int` (`/Game/TopDown/Blueprints/BP_Game.Difficulty Level` (`self.Game`)) :`0` 0 :`1` 1 :`2` 2 :`3` 3 :`4` 4)) 1))
      (`KismetArrayLibrary.Array_Add` (`self.Order`) (`.Result_2_28C2311B443FB4E495C6578C18E4F696` (break `/Game/TopDown/Items/S_Recipe` (`KismetArrayLibrary.Array_Random` (`/Game/TopDown/Blueprints/BP_TopDownGameMode.Get Available Recipes` _asbp_top_down_game_mode))))))))

(fn `Open Menu`
  (locals (Col :type "LinearColor Structure" :default (struct :`G` 0.405331 :`B` 0.050529 :`A` 1.0)))
  (bind _returnvalue (`GameplayStatics.GetPlayerController` 0))
  (`parent.Open Menu`)
  (bind _returnvalue_2 (`|CreateWidget` "/Game/UI/InventoryElements/WB_CalbackButton.WB_CalbackButton_C" null "Confirm Order"))
  (`Button.SetBackgroundColor` (`/Game/UI/InventoryElements/WB_CalbackButton.Mix` _returnvalue_2) (`local.Col`))
  (`self.Add Bottom Panel To Menu` _returnvalue_2)
  (add `/Game/UI/InventoryElements/WB_CalbackButton.Action` _returnvalue_2 (`|CreateDelegate` :!event `Confirm Order`))
  (bind _asbp_hud (cast `/Game/UI/BP_HUD` (`PlayerController.GetHUD` _returnvalue)))
  (bind _returnvalue_3 (`|CreateWidget` "/Game/UI/WB_OrderView.WB_OrderView_C" _returnvalue (`self.Order`)))
  (bind _output_get (set `self.OrderView` _returnvalue_3))
  (`PanelWidget.AddChild` (`/Game/UI/WB_HUD.Order` (`/Game/UI/BP_HUD.HUD` _asbp_hud)) _output_get))

(fn `UserConstructionScript`
  (`parent.UserConstructionScript`))