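; Pedestrian spawner actor that keeps a stream of BP_Customer characters walking from a Start point to an End point.
; A self-repeating SpawnLoop, started on BeginPlay, spawns each customer with a random max speed, sends it toward End, then waits a short random delay.
; A Box component destroys any customer that begins overlapping it.
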(event `SpawnLoop`
  (bind (_returnvalue_x _returnvalue_y) (`KismetMathLibrary.BreakVector` (`SceneComponent.K2_GetComponentLocation` (`self.End`))))
  (bind _returnvalue (`AIBlueprintHelperLibrary.SpawnAIFromClass` "/Game/TopDown/Blueprints/BP_Customer.BP_Customer_C" null (`SceneComponent.K2_GetComponentLocation` (`self.Start`)) (struct :`Yaw` 90.0) false null :!label _label))
  (bind _asbp_customer (cast `/Game/TopDown/Blueprints/BP_Customer` _returnvalue))
  (`/Game/TopDown/Blueprints/BP_Customer.SetMaxSpeed` _asbp_customer (`KismetMathLibrary.RandomFloatInRange` 150.0 400.0))
  (`/Game/TopDown/Blueprints/BP_Customer.EventMove` _asbp_customer (`KismetMathLibrary.MakeVector` _returnvalue_x _returnvalue_y))
  (`KismetSystemLibrary.Delay` (`KismetMathLibrary.RandomFloatInRange` 1.0 3.0))
  (`self.SpawnLoop`))

(event `self.ReceiveBeginPlay`
  (add `PrimitiveComponent.OnComponentBeginOverlap` (`self.Box`) (delegate `OnComponentBeginOverlap_Event`))
  (goto _label))

(event `OnComponentBeginOverlap_Event`
  (params (OverlappedComponent :type "PrimitiveComponent Object Reference") (OtherActor :type "Actor Object Reference") (OtherComp :type "PrimitiveComponent Object Reference") (OtherBodyIndex :type Integer) (bFromSweep :type Boolean) (SweepResult :type "HitResult Structure (by ref)"))
  (bind _asbp_customer (cast `/Game/TopDown/Blueprints/BP_Customer` OtherActor))
  (`self.K2_DestroyActor` _asbp_customer))

(fn `UserConstructionScript`)